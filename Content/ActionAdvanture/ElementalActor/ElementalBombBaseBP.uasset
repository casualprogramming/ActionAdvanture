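; Base Blueprint for an elemental bomb that reacts to fire and spreads an element when it explodes.
; Burn and extinguish events from its ElementalListener component toggle a FireEmitter hosted as a child actor.
; When its explosion component fires, a fixed-radius sphere overlap passes the explosion element to nearby listener actors, printing each one's name.
; The construction script sets the mesh's Color material parameter to white.
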(event `self.ReceiveBeginPlay`)

(event `self.ElementalListenerComp.OnBurn`
  (bind _asfire_emitter (cast `/Game/ActionAdvanture/ElementalActor/FireEmitter` (`ChildActorComponent.ChildActor` (`self.ChildActor`))))
  (`ElementalEmitter.ActivateEmitter` _asfire_emitter))

(event `self.ElementalListenerComp.OnExtinguished`
  (bind _asfire_emitter (cast `/Game/ActionAdvanture/ElementalActor/FireEmitter` (`ChildActorComponent.ChildActor` (`self.ChildActor`))))
  (`ElementalEmitter.DeactivateEmitter` _asfire_emitter))

(event `self.ExplosionComp.OnExploded`
  (params (OverlappedComponent :type "PrimitiveComponent Object Reference") (OtherActor :type "Actor Object Reference") (OtherComp :type "PrimitiveComponent Object Reference") (OtherBodyIndex :type Integer) (bFromSweep :type Boolean) (SweepResult :type "HitResult Structure (by ref)"))
  (bind _outactors (`KismetSystemLibrary.SphereOverlapActors` (`self.K2_GetActorLocation`) 200.0 (`self.ElementalListener`)))
  (for _array_element _outactors
    (`KismetSystemLibrary.PrintString` (`KismetSystemLibrary.GetObjectName` _array_element))
    (`ElementalListenerComponent.RecieveElement` (`self.GetComponentByClass` _array_element "/Script/ActionAdvanture.ElementalListenerComponent") (`self.ExplosionElementType`) null)))

(fn `UserConstructionScript`
  (`MeshComponent.SetVectorParameterValueOnMaterials` (`self.StaticMeshComp`) "Color" (1.0 1.0 1.0)))
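; Player character Blueprint that starts and stops a grab action through its ActionSystem from input.
; Pressing input action 1 calls NewFunction0 to start GrabActionBP, and input action 2 stops it directly.
; Both paths read the action name from the class via GetDefaultActionClass, then start or stop the action by that name.
; BeginPlay, Tick, overlap and the construction script are empty.
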(event `InputAction|1`
  (params (Key :type "Key Structure"))
  (:`Pressed`
    (`self.NewFunction_0` "/Game/ActionAdvanture/Action/GrabActionBP.GrabActionBP_C")))

(event `InputAction|2`
  (params (Key :type "Key Structure"))
  (:`Pressed`
    (bind _returnvalue (`NewBlueprintFunctionLibrary.GetDefaultActionClass` "/Game/ActionAdvanture/Action/GrabActionBP.GrabActionBP_C"))
    (`ActionSystemComponent.StopActionByName` (`self.ActionSystem`) (`Action.GetActionName` _returnvalue) null)))

(event `self.ReceiveTick`
  (params (DeltaSeconds :type "Float (single-precision)")))

(fn `NewFunction_0`
  (params (Class :type "Action Class Reference"))
  (bind _returnvalue (`NewBlueprintFunctionLibrary.GetDefaultActionClass` Class))
  (`ActionSystemComponent.StartActionByName` (`self.ActionSystem`) (`Action.GetActionName` _returnvalue) null))

(fn `UserConstructionScript`)
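; Player character Blueprint for an action-adventure game that maps inputs to abilities and what appear to be debug tests.
; Inputs start, cancel or stop grab, throw, projectile and melee actions on ActionSystemComp, resolving each name from its action class.
; Other keys spawn short-lived fire, water and ice emitters in front of the character.
; Test-style inputs also subtract HP through AttributeComp and broadcast a "Hello" event through the action system.
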(event `InputAction|1`
  (params (Key :type "Key Structure"))
  (:`Pressed`
    (bind _returnvalue (`NewBlueprintFunctionLibrary.GetDefaultActionName` "/Game/ActionAdvanture/PlayerCharacter/Action/PlayerGrab_Action.PlayerGrab_Action_C"))
    (`ActionSystemComponent.StartActionByName` (`self.ActionSystemComp`) _returnvalue null)))

(event `InputAction|2`
  (params (Key :type "Key Structure"))
  (:`Pressed`
    (bind _returnvalue (`NewBlueprintFunctionLibrary.GetDefaultActionName` "/Game/ActionAdvanture/PlayerCharacter/Action/PlayerGrab_Action.PlayerGrab_Action_C"))
    (`ActionSystemComponent.CancelActionByName` (`self.ActionSystemComp`) _returnvalue null)))

(event `self.ReceiveTick`
  (params (DeltaSeconds :type "Float (single-precision)")))

(event `InputAction|3`
  (params (Key :type "Key Structure"))
  (:`Pressed`
    (bind _returnvalue (`NewBlueprintFunctionLibrary.GetDefaultActionName` "/Game/ActionAdvanture/PlayerCharacter/Action/PlayerThrow_Action.PlayerThrow_Action_C"))
    (`ActionSystemComponent.StartActionByName` (`self.ActionSystemComp`) _returnvalue null)))

(event `InputAction|4`
  (params (Key :type "Key Structure"))
  (:`Pressed`
    (`AttributeComponent.SubtractHP` (`self.AttributeComp`) null 20.0)))

(event `InputAction|4`
  (params (Key :type "Key Structure"))
  (:`Pressed`
    (`ActionSystemComponent.BroadcastEvent` (`self.ActionSystemComp`) "Hello" (`self.GetOwner`))))

(event `InputAction|5`
  (params (Key :type "Key Structure"))
  (:`Pressed`
    (bind _returnvalue (`NewBlueprintFunctionLibrary.GetDefaultActionName` "/Game/ActionAdvanture/Action/MontageActions/ProjectileAction/ProjectTile_Action.ProjectTile_Action_C"))
    (`ActionSystemComponent.StartActionByName` (`self.ActionSystemComp`) _returnvalue null)))

(event `Key|Six`
  (params (Key :type "Key Structure"))
  (:`Pressed`
    (bind _returnvalue (`NewBlueprintFunctionLibrary.GetDefaultActionName` "/Game/ActionAdvanture/PlayerCharacter/Action/PlayerMeleeAttack_Action.PlayerMeleeAttack_Action_C"))
    (`ActionSystemComponent.StartActionByName` (`self.ActionSystemComp`) _returnvalue null)))

(event `Key|Seven`
  (params (Key :type "Key Structure"))
  (:`Pressed`
    (bind _returnvalue (`|SpawnActorFromClass` "/Game/ActionAdvanture/ElementalActor/FireEmitter.FireEmitter_C" (`KismetMathLibrary.MakeTransform` (+ (* (`self.GetActorForwardVector`) 50.0) (`self.K2_GetActorLocation`)) (`self.K2_GetActorRotation`) (3.0 3.0 3.0)) "Undefined" "OverrideRootScale" null null))
    (`self.SetLifeSpan` _returnvalue 4.0)))

(event `Key|Eight`
  (params (Key :type "Key Structure"))
  (:`Pressed`
    (bind _returnvalue (`|SpawnActorFromClass` "/Game/ActionAdvanture/ElementalActor/WaterSphereEmitter.WaterSphereEmitter_C" (`KismetMathLibrary.MakeTransform` (+ (* (`self.GetActorForwardVector`) 50.0) (`self.K2_GetActorLocation`)) (`self.K2_GetActorRotation`) (3.0 3.0 3.0)) "Undefined" "OverrideRootScale" null null))
    (`self.SetLifeSpan` _returnvalue 4.0)))

(event `Key|Nine`
  (params (Key :type "Key Structure"))
  (:`Pressed`
    (bind _returnvalue (`|SpawnActorFromClass` "/Game/ActionAdvanture/ElementalActor/IceSphereEmitter.IceSphereEmitter_C" (`KismetMathLibrary.MakeTransform` (+ (* (`self.GetActorForwardVector`) 50.0) (`self.K2_GetActorLocation`)) (`self.K2_GetActorRotation`) (3.0 3.0 3.0)) "Undefined" "OverrideRootScale" null null))
    (`self.SetLifeSpan` _returnvalue 4.0)))

(event `Key|T`
  (params (Key :type "Key Structure"))
  (bind _actionsystemcomp (`self.ActionSystemComp`))
  (:`Pressed`
    (bind _returnvalue (`NewBlueprintFunctionLibrary.GetDefaultActionName` "/Game/ActionAdvanture/PlayerCharacter/Action/GrabAndThrowVer2/PlayerGrab2_Action.PlayerGrab2_Action_C"))
    (`ActionSystemComponent.StartActionByName` _actionsystemcomp _returnvalue null))
  (:`Released`
    (`ActionSystemComponent.StopActionByName` _actionsystemcomp _returnvalue null)))

(fn `UserConstructionScript`)